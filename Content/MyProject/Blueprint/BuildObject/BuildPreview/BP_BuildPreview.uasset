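; Ghost preview actor for a build system that shows whether the chosen object can be placed at its current spot.
; On BeginPlay it takes the target class's default mesh and spawns a temporary instance to copy its snap point components.
; Each tick, two line traces require clear space above the origin and ground below the lower bound.
; That result and an overlap flag set CanBuild and the green or red material.
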(event `self.ReceiveBeginPlay`
  (`self.SetupPreview` (`self.ActorToSpawn`)))

(event `self.ReceiveTick`
  (params (DeltaSeconds :type "Float (single-precision)"))
  (bind _isvalid (`self.CheckGroundValidity`))
  (if (and _isvalid (not (`self.IsOverlappingPlayer?`)))
    (`PrimitiveComponent.SetMaterial` (`self.Preview`) 0 "/Game/MyProject/Mat/M_Ghost_Preview_Green.M_Ghost_Preview_Green")
    (set `self.CanBuild?` true)
    (else
      (`PrimitiveComponent.SetMaterial` (`self.Preview`) 0 "/Game/MyProject/Mat/M_Ghost_Preview_Red.M_Ghost_Preview_Red")
      (set `self.CanBuild?` false))))

(event `self.Preview.OnComponentBeginOverlap`
  (params (OverlappedComponent :type "PrimitiveComponent Object Reference") (OtherActor :type "Actor Object Reference") (OtherComp :type "PrimitiveComponent Object Reference") (OtherBodyIndex :type Integer) (bFromSweep :type Boolean) (SweepResult :type "HitResult Structure (by ref)"))
  (set `self.IsOverlappingPlayer?` true))

(event `self.Preview.OnComponentEndOverlap`
  (params (OverlappedComponent :type "PrimitiveComponent Object Reference") (OtherActor :type "Actor Object Reference") (OtherComp :type "PrimitiveComponent Object Reference") (OtherBodyIndex :type Integer))
  (set `self.IsOverlappingPlayer?` false))

(fn `CheckGroundValidity`
  (returns (IsValid :type Boolean))
  (bind _returnvalue (`self.K2_GetActorLocation`))
  (bind (_min _max) (`StaticMeshComponent.GetLocalBounds` (`self.Preview`)))
  (bind _returnvalue_2 (+ _min _returnvalue))
  (`|ExecutionSequence`
    (:`then_0`
      (bind (_outhit _returnvalue_3) (`KismetSystemLibrary.LineTraceSingle` (+ _max _returnvalue) _returnvalue "TraceTypeQuery1")))
    (:`then_1`
      (bind (_outhit_2 _returnvalue_4) (`KismetSystemLibrary.LineTraceSingle` _returnvalue_2 (- _returnvalue_2 (0.0 0.0 100.0)) "TraceTypeQuery1")))
    (:`then_2`
      (return (and (not _returnvalue_3) _returnvalue_4)))))

(fn `SetupPreview`
  (params (TargetClass :type "/Game/MyProject/Blueprint/BuildObject/BuildBase/BP_BuildBase Class Reference"))
  (for _array_element (`self.K2_GetComponentsByClass` "/Game/MyProject/Blueprint/BuildObject/BPC_SnapPoint.BPC_SnapPoint_C")
    (`ActorComponent.K2_DestroyComponent` _array_element))
  (`StaticMeshComponent.SetStaticMesh` (`self.Preview`) (defaults `Object` TargetClass))
  (bind _returnvalue (`|SpawnActorFromClass` TargetClass (`KismetMathLibrary.MakeTransform` (0.0 0.0 0.0)) "Undefined" "MultiplyWithRoot" null null))
  (for _array_element_2 (`self.K2_GetComponentsByClass` _returnvalue "/Game/MyProject/Blueprint/BuildObject/BPC_SnapPoint.BPC_SnapPoint_C")
    (`|AddComponentByClass` "/Game/MyProject/Blueprint/BuildObject/BPC_SnapPoint.BPC_SnapPoint_C" false (`SceneComponent.GetRelativeTransform` _array_element_2)))
  (`self.K2_DestroyActor` _returnvalue))

(fn `UserConstructionScript`)