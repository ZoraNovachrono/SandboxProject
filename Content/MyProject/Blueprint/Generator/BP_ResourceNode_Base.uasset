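; BP_ResourceNode_Base is a harvestable resource node that gives the player items each time it is hit and respawns after depletion.
; Each hit lowers health and spawns a BP_GrabItem carrying the resource type and per-hit quantity, passed straight to the first-person character's GrabItem.
; At zero health it hides its mesh and disables collision, then restores both and refills health after a respawn delay.
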(event `self.ReceiveBeginPlay`
  (set `self.Health` (`self.MaxHealth`)))

(event `OnHit`
  (params (Damage :type Integer))
  (bind _health (`self.Health`))
  ; Reduce health and give ressources to player
  (set `self.Health` (- (`self.Health`) Damage))
  (bind _asbp_first_person_character (cast `/Game/FirstPerson/Blueprints/BP_FirstPersonCharacter` (`GameplayStatics.GetPlayerCharacter` 0)))
  (bind _returnvalue (`|SpawnActorFromClass` "/Game/MyProject/Blueprint/GrabObject/BP_GrabItem.BP_GrabItem_C" (`KismetMathLibrary.MakeTransform` (0.0 0.0 0.0)) "Undefined" "MultiplyWithRoot" null null))
  (`|ExecutionSequence`
    (:`then_0`
      (set `/Game/MyProject/Blueprint/GrabObject/BP_GrabItem.ItemRow` (`self.ResourceType`) _returnvalue))
    (:`then_1`
      (set `/Game/MyProject/Blueprint/GrabObject/BP_GrabItem.Item Quantity` (`self.QuantityPerHit`) _returnvalue))
    (:`then_2`
      (`/Game/FirstPerson/Blueprints/BP_FirstPersonCharacter.Grab Item` _asbp_first_person_character _returnvalue)
      (if (<= _health 0)
        ; Disable de generator and enable it after delay
        (`SceneComponent.SetVisibility` (`self.StaticMesh`) false false)
        (`self.SetActorEnableCollision` false)
        (`KismetSystemLibrary.Delay` (`self.RespawnTime`))
        (set `self.Health` (`self.MaxHealth`))
        (`SceneComponent.SetVisibility` (`self.StaticMesh`) true false)
        (`self.SetActorEnableCollision` true)
        (else
          (`KismetSystemLibrary.PrintString` (`KismetStringLibrary.Concat_StrStr` "Ressource touchée ! Vie restante :" (`KismetStringLibrary.Conv_IntToString` _health))))))))

(fn `UserConstructionScript`)