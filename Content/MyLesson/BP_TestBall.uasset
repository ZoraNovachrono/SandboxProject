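; BP_TestBall is a physics test ball that appears to check whether a fast sphere tunnels through obstacles with or without CCD.
; On BeginPlay it applies the UseCCD flag to the Sphere and launches it along the actor's forward vector at LaunchSpeed.
; Hit sets HasHit and prints the speed; without a hit after a short delay, BeginPlay prints it.
; Both cases print the same "TRAVERSÉ" (passed through) label.
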(event `self.ReceiveBeginPlay`
  (`PrimitiveComponent.SetUseCCD` (`self.Sphere`) (`self.UseCCD `) "None")
  (`PrimitiveComponent.SetPhysicsLinearVelocity` (`self.Sphere`) (* (`self.GetActorForwardVector`) (`self.LaunchSpeed `)) false "None")
  (`KismetSystemLibrary.Delay` 1.0)
  (if (not (`self.HasHit `))
    (`KismetSystemLibrary.PrintString` (`KismetStringLibrary.Concat_StrStr` "TRAVERSÉ  : " (`KismetStringLibrary.Conv_DoubleToString` (`KismetMathLibrary.VSize` (`self.GetVelocity`)))))))

(event `self.ReceiveHit`
  (params (MyComp :type "PrimitiveComponent Object Reference") (Other :type "Actor Object Reference") (OtherComp :type "PrimitiveComponent Object Reference") (bSelfMoved :type Boolean) (HitLocation :type "Vector Structure") (HitNormal :type "Vector Structure") (NormalImpulse :type "Vector Structure") (Hit :type "HitResult Structure (by ref)"))
  (set `self.HasHit ` true)
  (`KismetSystemLibrary.PrintString` (`KismetStringLibrary.Concat_StrStr` "TRAVERSÉ  : " (`KismetStringLibrary.Conv_DoubleToString` (`KismetMathLibrary.VSize` (`self.GetVelocity`))))))

(fn `UserConstructionScript`)